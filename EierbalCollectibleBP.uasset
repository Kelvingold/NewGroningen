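; EierbalCollectible is a pickup that animates in place and scores a point when something overlaps its box.
; A looping Timeline lerps the model between its current position and a point below it, restarted from Tick through a cooldown flag.
; Tick also adds a fixed, frame-rate-dependent yaw step for spin.
; The first overlap calls PointScored on the PointsCounter actor, spawns confetti and destroys the collectible.
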(event `self.ReceiveBeginPlay`
  (bind _eierbalmodel (`self.EierbalModel`))
  (bind (_returnvalue_x _returnvalue_y _returnvalue_z) (`KismetMathLibrary.BreakVector` (`SceneComponent.K2_GetComponentLocation` _eierbalmodel)))
  (set `self.AnimationCooldown` true)
  (set `self.PositionA` (`SceneComponent.K2_GetComponentLocation` _eierbalmodel) :!label _label)
  (set `self.PositionB` (`KismetMathLibrary.MakeVector` _returnvalue_x _returnvalue_y (- _returnvalue_z 25.0)))
  (bind (_direction _floattrack02) (`Timeline|Timeline` :!via `PlayFromStart`)
    (:`Update`
      (`SceneComponent.K2_SetWorldLocation` (`self.EierbalModel`) (`KismetMathLibrary.VLerp` (`self.PositionA`) (`self.PositionB`) _floattrack02) false false))
    (:`Finished`
      (set `self.AnimationCooldown` false))))

(event `self.ReceiveTick`
  (params (DeltaSeconds :type "Float (single-precision)"))
  (bind _eierbalmodel (`self.EierbalModel`))
  (bind (_returnvalue_roll _returnvalue_pitch _returnvalue_yaw) (`KismetMathLibrary.BreakRotator` (`SceneComponent.K2_GetComponentRotation` _eierbalmodel)))
  (`|ExecutionSequence`
    (:`then_0`
      (if (not (`self.AnimationCooldown`))
        (set `self.AnimationCooldown` true)
        (goto _label)))
    (:`then_1`
      (`SceneComponent.K2_SetWorldRotation` _eierbalmodel (`KismetMathLibrary.MakeRotator` _returnvalue_roll _returnvalue_pitch (+ _returnvalue_yaw 2.0)) false false))))

(event `self.Box.OnComponentBeginOverlap`
  (params (OverlappedComponent :type "PrimitiveComponent Object Reference") (OtherActor :type "Actor Object Reference") (OtherComp :type "PrimitiveComponent Object Reference") (OtherBodyIndex :type Integer) (bFromSweep :type Boolean) (SweepResult :type "HitResult Structure (by ref)"))
  (`/Engine/EditorBlueprintResources/StandardMacros.DoOnce` false
    (:`Completed`
      (bind _returnvalue (`GameplayStatics.GetActorOfClass` "/Game/Blueprints/PointsCounter.PointsCounter_C"))
      (`/Game/Blueprints/PointsCounter.PointScored` _returnvalue)
      (`NiagaraFunctionLibrary.SpawnSystemAtLocation` "/Game/ParticleSystems/ParticleConfetti.ParticleConfetti" (`self.K2_GetActorLocation`))
      (`self.K2_DestroyActor`))))

(fn `UserConstructionScript`)